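; BP_TimePlus is a time-bonus pickup that extends the time in the time-out game mode.
; It overrides the parent's PickUp event, runs the parent logic, then casts the game mode to BP_TimeOutGameMode and adds a fixed amount to ExistingTime.
; The BeginPlay, overlap and Tick events are disabled stubs, so any triggering comes from outside this graph.
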(event `self.PickUp`
  (`parent.PickUp`)
  (bind _asbp_time_out_game_mode (cast `/Game/DevKang/Blueprints/GameBP/BP_TimeOutGameMode` (`GameplayStatics.GetGameMode`)))
  (set `/Game/DevKang/Blueprints/GameBP/BP_TimeOutGameMode.ExistingTime` (+ (`/Game/DevKang/Blueprints/GameBP/BP_TimeOutGameMode.ExistingTime` _asbp_time_out_game_mode) 10.0) _asbp_time_out_game_mode))

(fn `UserConstructionScript`
  (`parent.UserConstructionScript`))