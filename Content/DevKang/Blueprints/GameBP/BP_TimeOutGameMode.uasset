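; BP_TimeOutGameMode is a timed game mode that ends in a Clear or Failed result based on a count of BP_pongtree actors.
; BeginPlay sets game-only input and records how many trees are in the level as FullCount.
; Tick counts down ExistingTime, then a DoOnce compares Count, which is not modified here, with FullCount.
; It shows the verdict in WB_Result and switches to UI-only input with a visible cursor.
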(event `self.ReceiveBeginPlay`
  (bind _returnvalue (`GameplayStatics.GetPlayerController` 0))
  (`WidgetBlueprintLibrary.SetInputMode_GameOnly` _returnvalue)
  (set `PlayerController.bShowMouseCursor` false _returnvalue)
  (bind _outactors (`GameplayStatics.GetAllActorsOfClass` "/Game/DevKang/Blueprints/Lectureonly/BP_pongtree.BP_pongtree_C"))
  (set `self.FullCount` (`KismetArrayLibrary.Array_Length` _outactors)))

(event `self.ReceiveTick`
  (params (DeltaSeconds :type "Float (single-precision)"))
  (bind _returnvalue (`GameplayStatics.GetPlayerController` 0))
  (bind _existingtime (`self.ExistingTime`))
  (bind _returnvalue_2 (- _existingtime DeltaSeconds))
  (set `self.ExistingTime` (`KismetMathLibrary.FClamp` _returnvalue_2 0.0 _existingtime))
  (if (<= _returnvalue_2 0.0)
    (`/Engine/EditorBlueprintResources/StandardMacros.DoOnce` false
      (:`Completed`
        (if (== (`self.Count`) (`self.FullCount`))
          (set `self.ResultMessage` "Clear")
          (else
            (set `self.ResultMessage` "Failed")))
        (bind _returnvalue_3 (`|CreateWidget` "/Game/DevKang/Widget/WB_Result.WB_Result_C"))
        (`TextBlock.SetText` (`/Game/DevKang/Widget/WB_Result.WidgetDisplay` _returnvalue_3) (`self.ResultMessage`))
        (`UserWidget.AddToViewport` _returnvalue_3 0)
        (`WidgetBlueprintLibrary.SetInputMode_UIOnlyEx` _returnvalue null "LockAlways")
        (set `PlayerController.bShowMouseCursor` true _returnvalue)))))

(fn `UserConstructionScript`)