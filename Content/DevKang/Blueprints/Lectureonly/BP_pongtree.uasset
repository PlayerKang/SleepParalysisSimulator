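; BP_pongtree is a clickable tree actor for a timeout counting minigame, shown through its Plane component.
; On BeginPlay the Plane becomes visible.
; GetClicked increments Count on BP_TimeOutGameMode, then hides the Plane and sets it to ignore the Visibility channel so click traces no longer hit it.
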(event `self.ReceiveBeginPlay`
  (`SceneComponent.SetVisibility` (`self.Plane`) true false))

(event `GetClicked`
  (bind _plane (`self.Plane`))
  (bind _asbp_time_out_game_mode (cast `/Game/DevKang/Blueprints/GameBP/BP_TimeOutGameMode` (`GameplayStatics.GetGameMode`)))
  (set `/Game/DevKang/Blueprints/GameBP/BP_TimeOutGameMode.Count` (+ (`/Game/DevKang/Blueprints/GameBP/BP_TimeOutGameMode.Count` _asbp_time_out_game_mode) 1) _asbp_time_out_game_mode)
  (`SceneComponent.SetVisibility` _plane false false)
  (`PrimitiveComponent.SetCollisionResponseToChannel` _plane "ECC_Visibility" "ECR_Ignore"))

(fn `UserConstructionScript`)