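; BP_Door is a door that swings open automatically when the player character enters its trigger box and closes when the player leaves.
; A timeline drives the door mesh's relative yaw up to a quarter turn, playing on overlap begin and reversing on overlap end.
; If an Interaction actor reference is valid, it is shown while the player is inside the box and hidden on exit.
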(event `self.Box.OnComponentBeginOverlap`
  (params (OverlappedComponent :type "PrimitiveComponent Object Reference") (OtherActor :type "Actor Object Reference") (OtherComp :type "PrimitiveComponent Object Reference") (OtherBodyIndex :type Integer) (bFromSweep :type Boolean) (SweepResult :type "HitResult Structure (by ref)"))
  (bind _interaction (`self.Interaction`))
  (cast `/Game/DevKang/Blueprints/GameBP/BP_PlayerCharacter` OtherActor)
  (`/Engine/EditorBlueprintResources/StandardMacros.IsValid` _interaction
    (:`Is Valid`
      (`self.SetActorHiddenInGame` _interaction false)
      (bind (_direction `_새_트랙_0`) (`Timeline|타임라인` :!label _label)
        (:`Update`
          (`SceneComponent.K2_SetRelativeRotation` (`self.SM_Door`) (`KismetMathLibrary.MakeRotator` 0.0 0.0 (* `_새_트랙_0` 90.0)) false false))))
    (:`Is Not Valid`
      (goto _label))))

(event `self.Box.OnComponentEndOverlap`
  (params (OverlappedComponent :type "PrimitiveComponent Object Reference") (OtherActor :type "Actor Object Reference") (OtherComp :type "PrimitiveComponent Object Reference") (OtherBodyIndex :type Integer))
  (bind _interaction (`self.Interaction`))
  (cast `/Game/DevKang/Blueprints/GameBP/BP_PlayerCharacter` OtherActor)
  (`/Engine/EditorBlueprintResources/StandardMacros.IsValid` _interaction
    (:`Is Valid`
      (`self.SetActorHiddenInGame` _interaction true)
      (goto _label :!via `Reverse`))
    (:`Is Not Valid`
      (goto _label :!via `Reverse`))))

(fn `UserConstructionScript`)